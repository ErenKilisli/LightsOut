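; BP_NPC is an NPC that attacks automatically when the game mode signals that the draw phase has started.
; On BeginPlay it runs the parent logic, then binds its handler to the game mode's DrawPhaseStarted event.
; The handler waits a random 0.3 to 1 second, acting as a reaction time, before calling Attack.
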(event `self.ReceiveBeginPlay`
  (`parent.ReceiveBeginPlay`)
  (add `/Game/Blueprints/GM_Duel.DrawPhaseStarted` (`self.gamemoderef`) (delegate `ondrawohaseStarted`)))

(event `ondrawohaseStarted`
  (`KismetSystemLibrary.Delay` (`KismetMathLibrary.RandomFloatInRange` 0.3 1.0))
  (`self.Attack`))

(fn `UserConstructionScript`
  (`parent.UserConstructionScript`))