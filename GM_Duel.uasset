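; Game mode for a reflex duel between the player car and an NPC car, cycling through Intro, Wait, Draw and Finish phases.
; Tick times the intro, waits a random delay, then enters Draw, broadcasts it and shows the BP_Exc signal actor.
; AttackedSuccesfully defeats the loser, shows a win or lose widget, records reaction time on player wins and starts a restart timer.
; Reset returns both cars and the phase to the start.
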(event `self.ReceiveBeginPlay`
  (bind _returnvalue (`GameplayStatics.GetActorOfClass` "/Game/Blueprints/BP_Exc.BP_Exc_C"))
  (set `self.Exc_Ref` _returnvalue)
  (bind _returnvalue_2 (`GameplayStatics.GetActorOfClass` "/Game/Blueprints/BP_playercar.BP_playercar_C"))
  (set `self.playerRef` _returnvalue_2)
  (bind _returnvalue_3 (`GameplayStatics.GetActorOfClass` "/Game/Blueprints/BP_carNPC.BP_carNPC_C"))
  (set `self.npc_refcar` _returnvalue_3))

(event `self.ReceiveTick`
  (params (DeltaSeconds :type "Float (single-precision)"))
  (set `self.ElapsedTime` (+ DeltaSeconds (`self.ElapsedTime`)))
  (switch `/Game/Blueprints/Enums/E_Phase` (`self.Phase`)
    (:`NewEnumerator0`
      (if (>= (`self.ElapsedTime`) (`self.RoundstartTime`))
        (set `self.Phase` "NewEnumerator1")
        (bind _output_get (set `self.drawDelay` (`KismetMathLibrary.RandomFloatInRange` (`self.MinDrawDelay`) (`self.MaxDrawDelay`))))
        (`KismetSystemLibrary.Delay` _output_get)
        (set `self.drawTime` (+ _output_get (`self.drawDelay`)))
        (set `self.Phase` "NewEnumerator2")
        (`self.DrawPhaseStarted`)
        (`/Engine/EditorBlueprintResources/StandardMacros.IsValid` (`self.Exc_Ref`)
          (:`Is Valid`
            (`/Game/Blueprints/BP_Exc.SetVisibility` (`self.Exc_Ref`) true))
          (:`Is Not Valid`
            (`KismetSystemLibrary.PrintString` "excNNOTfound")))))))

(fn `AttackedSuccesfully`
  (params (IsPlayer :type Boolean))
  (bind _exc_ref (`self.Exc_Ref`))
  (if IsPlayer
    (`/Game/Blueprints/BP_Samurai.Defeated` (`self.npc_refcar`))
    (set `self.reflexesTime` (- (`self.ElapsedTime`) (`self.drawTime`)))
    (bind _returnvalue (`|CreateWidget` "/Game/Blueprints/ui/YOUWIN.YOUWIN_C"))
    (bind _output_get (set `self.winscreen` _returnvalue))
    (`UserWidget.AddToViewport` _output_get 0)
    (else
      (`/Game/Blueprints/BP_Samurai.Defeated` (`self.playerRef`))
      (bind _returnvalue_2 (`|CreateWidget` "/Game/Blueprints/ui/YOULOSE.YOULOSE_C"))
      (bind _output_get_2 (set `self.losescreen` _returnvalue_2))
      (`UserWidget.AddToViewport` _output_get_2 0)))
  (`/Engine/EditorBlueprintResources/StandardMacros.IsValid` _exc_ref
    (:`Is Valid`
      (`/Game/Blueprints/BP_Exc.SetVisibility` _exc_ref false)
      (`KismetSystemLibrary.K2_SetTimerDelegate` (`|CreateDelegate` :!event `Reset`) (`self.RestartDElay`)))))

(fn `Reset`
  (set `self.Phase` "NewEnumerator0")
  (set `self.ElapsedTime` 0.0)
  (`/Game/Blueprints/BP_Samurai.Reset` (`self.playerRef`))
  (`/Game/Blueprints/BP_Samurai.Reset` (`self.npc_refcar`)))

(fn `SetGameFinished`
  (set `self.Phase` "NewEnumerator3"))

(fn `UserConstructionScript`)