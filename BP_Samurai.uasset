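; BP_Samurai is a duelist in a quick-draw game, sliding its sprite in at BeginPlay and on reset, and creating start screen and HUD widgets.
; Attack acts once per round based on GM_Duel's phase: pressing during Wait shows a cross, while Draw ends the game and plays a fast lunge timeline.
; That timeline's event swaps in the attack sprite and reports the hit to the game mode, flagging whether the attacker is player-controlled.
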(event `self.ReceiveBeginPlay`
  (bind _asgm_duel (cast `/Game/Blueprints/GM_Duel` (`GameplayStatics.GetGameMode`)))
  (set `self.gamemoderef` _asgm_duel)
  (set `self.sprite def Location` (`SceneComponent.RelativeLocation` (`self.PaperSprite`)))
  (`self.SlideIn`)
  (`self.setcrossvisibility` false)
  (bind _returnvalue (`|CreateWidget` "/Game/Blueprints/ui/startingscreen.startingscreen_C"))
  (bind _output_get (set `self.startscreen` _returnvalue))
  (`UserWidget.AddToViewport` _output_get 0)
  (`KismetSystemLibrary.Delay` 3.0)
  (bind _returnvalue_2 (`|CreateWidget` "/Game/Blueprints/ui/hud.hud_C"))
  (bind _output_get_2 (set `self.hud` _returnvalue_2))
  (`UserWidget.AddToViewport` _output_get_2 0))

(event `SlideIn`
  (`TimelineComponent.SetPlayRate` (`self.SlideInTimeline`) 2.0)
  (bind (_direction _alpha) (`Timeline|SlideInTimeline` :!via `PlayFromStart`)
    (:`Update`
      (`SceneComponent.K2_SetRelativeLocation` (`self.PaperSprite`) (`KismetMathLibrary.VLerp` (`self.slide start pos`) (`self.sprite def Location`) _alpha) false false))))

(event `Attack`
  (if (not (`self.PressedDraw?`))
    (switch `/Game/Blueprints/Enums/E_Phase` (`/Game/Blueprints/GM_Duel.Phase` (`self.gamemoderef`))
      (:`NewEnumerator1`
        (`self.setcrossvisibility` true)
        (set `self.PressedDraw?` true))
      (:`NewEnumerator2`
        (set `self.PressedDraw?` true)
        (`/Game/Blueprints/GM_Duel.SetGameFinished` (`self.gamemoderef`))
        (`TimelineComponent.SetPlayRate` (`self.AttaackTimeline`) 8.0)
        (bind (_direction _attacktrack) (`Timeline|AttaackTimeline` :!via `PlayFromStart`)
          (:`Update`
            (`SceneComponent.K2_SetRelativeLocation` (`self.PaperSprite`) (`KismetMathLibrary.VLerp` (`self.sprite def Location`) (`SceneComponent.RelativeLocation` (`self.AttackPso`)) _attacktrack) false false))
          (:`switchsprite`
            (`self.SetAttackSprite` (`self.Attack Sprite`))
            (`/Game/Blueprints/GM_Duel.AttackedSuccesfully` (`self.gamemoderef`) (`self.IsPlayerControlled`))))))))

(event `Defeated`
  (`PaperSpriteComponent.SetSprite` (`self.PaperSprite`) (`self.DefeatSprite`))
  (`self.setcrossvisibility` false))

(fn `Reset`
  (`PaperSpriteComponent.SetSprite` (`self.PaperSprite`) (`self.IdleSprite`))
  (set `self.PressedDraw?` false)
  (`self.SlideIn`))

(fn `SetAttackSprite`
  (params (AttackSprite :type "PaperSprite Object Reference"))
  (bind _papersprite (`self.PaperSprite`))
  (`PaperSpriteComponent.SetSprite` _papersprite AttackSprite)
  (`PrimitiveComponent.SetMaterial` _papersprite 0 "/Paper2D/TranslucentUnlitSpriteMaterial.TranslucentUnlitSpriteMaterial")
  (`PrimitiveComponent.SetTranslucentSortPriority` _papersprite 1))

(fn `setcrossvisibility`
  (params (bNewVisibility :type Boolean))
  (`SceneComponent.SetVisibility` (`self.cross`) bNewVisibility false))

(fn `UserConstructionScript`)